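; Ascila character Blueprint, mostly a thin layer of debug key bindings over functions defined outside this graph.
; Enter and R share a FlipFlop toggling slow motion, F and G exit and enter RMState, and Left Ctrl toggles controller-driven yaw.
; Bow spawning and socket attachment, HUD widget creation and ledge trace calls are present but unwired, so they never run.
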(event EventBeginPlay)

(event Collision|EventActorBeginOverlap
  (params (OtherActor :type Actor%20Object%20Reference)))

(event EventTick
  (params (DeltaSeconds :type Float%20%28single-precision%29)))

(event Input|KeyboardEvents|Enter
  (params (Key :type Key%20Structure :default "None"))
  ;[0 1 0.1797] Utilities _ test
  (:Pressed
    (Utilities|FlowControl|FlipFlop
      (:A
        (Development|ExecuteConsoleCommand "slomo 0.1" 0))
      (:B
        (Development|ExecuteConsoleCommand "slomo 1" 0)))))

(event Input|KeyboardEvents|R
  (params (Key :type Key%20Structure :default "None"))
  ;[0 1 0.1797] Utilities _ test
  (:Pressed
    (Utilities|FlowControl|FlipFlop
      (:A
        (Development|ExecuteConsoleCommand "slomo 0.1" 0))
      (:B
        (Development|ExecuteConsoleCommand "slomo 1" 0)))))

(event Input|KeyboardEvents|LeftCtrl
  (params (Key :type Key%20Structure :default "None"))
  ;[0 1 0.1797] Utilities _ test
  (:Pressed
    (Utilities|FlowControl|FlipFlop
      (:A
        (Variables|Default|SetbUseControllerRotationYaw false))
      (:B
        (Variables|Default|SetbUseControllerRotationYaw true)))))

(event Input|KeyboardEvents|F
  (params (Key :type Key%20Structure :default "None"))
  ;[0 1 0.1797] Utilities _ test
  (:Pressed
    (Class|ATHAscila|ExitRMState)))

(event Input|KeyboardEvents|G
  (params (Key :type Key%20Structure :default "None"))
  ;[0 1 0.1797] Utilities _ test
  (:Pressed
    (Class|ATHAscila|EnterRMState)))

(fn ConstructionScript)