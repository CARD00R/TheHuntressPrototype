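; Render-target actor for the reactive snow showcase, managing a scene capture area and a persistent snow render target.
; On BeginPlay it shares the capture width with MPC_Snow, clears both targets, then repeatedly draws MAT_DrawToPersistent into RT_Persistent on a fast looping timer.
; MoveRenderTarget shifts the actor to the player's XY, snapped to the capture's texel grid, and writes the new location to MPC_Snow.
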(event Custom|DrawToRT
  (Rendering|DrawMaterialtoRenderTarget "/Game/Maps/Showcase/BasicPlayerLocomotion/ReactiveSnow/RT_Persistent.RT_Persistent" (Variables|Default|GetDrawToPMat)))

(event Custom|MoveRenderTarget
  (bind _returnvalue (Transformation|GetActorLocation))
  (bind _returnvalue_2 (Game|GetPlayerCharacter 0))
  (bind _returnvalue_3 (/ 1.0 256.0))
  (bind _scenecapturecomponent2d (Variables|Default|GetSceneCaptureComponent2D))
  (bind _returnvalue_4 (Transformation|GetActorLocation _returnvalue_2))
  (bind _orthowidth (Variables|/Script/Engine.SceneCaptureComponent2D|GetOrthoWidth _scenecapturecomponent2d))
  (bind _returnvalue_5 (* _orthowidth _returnvalue_3))
  (bind _returnvalue_6 (Utilities|SnapPixeltoGrid (.x _returnvalue_4) _returnvalue_5 (.y _returnvalue_4)))
  (bind _returnvalue_7 (- _returnvalue_6 _returnvalue))
  (bind _output_get (Variables|Default|SetMoveOffSet (Math|Vector2D|MakeVector2D (.x _returnvalue_7) (.y _returnvalue_7))))
  (Transformation|AddActorWorldOffset (Math|Vector|MakeVector (.x _output_get) (.y _output_get) 0.0))
  (Rendering|Material|SetVectorParameterValue "/Game/Maps/Showcase/BasicPlayerLocomotion/ReactiveSnow/MPC_Snow.MPC_Snow" "CaptureLocation" (Math|Conversions|ToLinearColor(Vector) (Transformation|GetActorLocation)) :!class /Script/Engine.KismetMaterialLibrary))

(event EventBeginPlay
  (Utilities|FlowControl|Sequence
    (:then_0
      (Rendering|Material|SetScalarParameterValue "/Game/Maps/Showcase/BasicPlayerLocomotion/ReactiveSnow/MPC_Snow.MPC_Snow" "Size" (Variables|/Script/Engine.SceneCaptureComponent2D|GetOrthoWidth (Variables|Default|GetSceneCaptureComponent2D)) :!class /Script/Engine.KismetMaterialLibrary)
      (bind _returnvalue (Rendering|Material|CreateDynamicMaterialInstance "/Game/Maps/Showcase/BasicPlayerLocomotion/ReactiveSnow/MAT_DrawToPersistent.MAT_DrawToPersistent" "None" :!class /Script/Engine.KismetMaterialLibrary))
      (Variables|Default|SetDrawToPMat _returnvalue)
      (Rendering|ClearRenderTarget2D "/Game/Maps/Showcase/BasicPlayerLocomotion/ReactiveSnow/RT_RenderTarget.RT_RenderTarget")
      (Rendering|ClearRenderTarget2D "/Game/Maps/Showcase/BasicPlayerLocomotion/ReactiveSnow/RT_Persistent.RT_Persistent"))
    (:then_1
      ;[0 0.8828 1] Do it in tick for better quality lower performance
      (Utilities|Time|SetTimerbyEvent (delegate Custom|DrawToRT) 0.01 true))))

(fn ConstructionScript)