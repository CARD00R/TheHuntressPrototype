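; BP_CameraChanger is a level trigger volume that switches the player's camera framing when BP_Ascila enters its box.
; On overlap, the SetTo value selects a preset of distance, FOV, offset and transition speed, passed to the character's ChangeCameraProperties.
; The first preset also turns off controller-yaw rotation, and no other preset restores it.
; BeginPlay caches a BP_Knight_General reference that the visible logic never uses.
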(event OnComponentBeginOverlap(Box)
  (params (OverlappedComponent :type Primitive%20Component%20Object%20Reference) (OtherActor :type Actor%20Object%20Reference) (OtherComp :type Primitive%20Component%20Object%20Reference) (OtherBodyIndex :type Integer) (bFromSweep :type Boolean) (SweepResult :type Hit%20Result%20Structure%20%28by%20ref%29))
  (bind _asbp_ascila (Utilities|Casting|CastToBP_Ascila OtherActor))
  (switch int (Variables|Default|GetSetTo)
    (:0
      (Variables|/Script/Engine.Pawn|SetbUseControllerRotationYaw _asbp_ascila false)
      (Class|ATHAscila|ChangeCameraProperties _asbp_ascila 1e+03 9e+01 "0,55.000000,-305.000000" 0.02))
    (:1
      (Class|ATHAscila|ChangeCameraProperties _asbp_ascila 4e+02 9e+01 "0.000000,55.000000,80.000000" 0.02))
    (:2
      (Class|ATHAscila|ChangeCameraProperties _asbp_ascila 5.5e+02 9e+01 "0.000000,340.000000,80.000000" 0.02))
    (:3
      ;[1 0.2812 0] Default
      (Class|ATHAscila|ChangeCameraProperties _asbp_ascila 4e+02 9e+01 "0.000000,55.000000,80.000000" 0.01))))

(event EventBeginPlay
  (bind _returnvalue (Actor|GetActorOfClass "/Game/Maps/Showcase/BasicPlayerLocomotion/Knights/WithOut/Anim/BP/General/BP_Knight_General.BP_Knight_General_C"))
  (Variables|Default|SetGeneral _returnvalue))

(event Collision|EventActorBeginOverlap
  (params (OtherActor :type Actor%20Object%20Reference)))

(event EventTick
  (params (DeltaSeconds :type Float%20%28single-precision%29)))

(fn ConstructionScript)